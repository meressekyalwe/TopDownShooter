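; Weapon pickup actor for the top-down shooter, offered to a character's inventory on overlap.
; BeginPlay initializes mesh and particles from WeaponInfo, querying the game instance's drop-item info only when ItemName is None, and removes unneeded components.
; A successful inventory add completes the pickup; otherwise the character starts a weapon switch, which ends when leaving the sphere.
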(event OnComponentEndOverlap(Sphere)
  (params (OverlappedComponent :type Primitive%20Component%20Object%20Reference) (OtherActor :type Actor%20Object%20Reference) (OtherComp :type Primitive%20Component%20Object%20Reference) (OtherBodyIndex :type Integer))
  (bind _asbp_top_down_shooter_character (Utilities|Casting|CastToBP_TopDownShooterCharacter OtherActor))
  (Default|EndSwitchWeapon _asbp_top_down_shooter_character))

(event EventBeginPlay
  (bind _itemname (Variables|Default|GetItemName))
  (|CallParentFunction)
  (if (Utilities|Name|Equal(Name) _itemname "None")
    (bind _asbp_game_instance (Utilities|Casting|CastToBP_GameInstance (Game|GetGameInstance)))
    (bind (_outinfo _returnvalue) (Class|TopDownShooterGameInstance|GetDropItemInfobyName _asbp_game_instance _itemname))
    (if _returnvalue
      (Variables|Default|SetWeaponInfo _outinfo)))
  (CallFunction|InitActor (Variables|Default|GetWeaponInfo)))

(event Collision|EventActorBeginOverlap
  (params (OtherActor :type Actor%20Object%20Reference))
  (|CallParentFunction OtherActor) ; This node is disabled and will not be called.\nDrag off pins to build functionality.
)

(event EventTick
  (params (DeltaSeconds :type Float%20%28single-precision%29))
  (|CallParentFunction DeltaSeconds) ; This node is disabled and will not be called.\nDrag off pins to build functionality.
)

(event EventOverlapCharacter
  (params (ToInventory :type Top%20Down%20Shooter%20Inventor%20Component%20Object%20Reference))
  (|CallParentFunction ToInventory)
  (bind _returnvalue (Class|TopDownShooterInventorComponent|TryGetWeapontoInventory ToInventory (.WeaponInfo (Utilities|Struct|BreakDropItem (Variables|Default|GetWeaponInfo)))))
  (if _returnvalue
    (Default|PickUpSucces self)
    (else
      (bind _asbp_top_down_shooter_character (Utilities|Casting|CastToBP_TopDownShooterCharacter (Components|GetOwner ToInventory)))
      (Default|StartSwitchWeapon _asbp_top_down_shooter_character self))))

(fn ConstructionScript
  (|CallParentFunction))

(fn InitActor
  (params (InfoActor :type Drop%20Item%20Structure))
  (bind (_weaponstaticmesh _weaponskeletmesh _particlesystem _offset _weaponinfo) (Utilities|Struct|BreakDropItem InfoActor))
  (bind _staticmesh (Variables|Default|GetStaticMesh))
  (bind _skeletalmesh (Variables|Default|GetSkeletalMesh))
  (bind _particlesystem_2 (Variables|Default|GetParticleSystem))
  (bind (_location _rotation _scale) (Math|Transform|BreakTransform _offset))
  (Utilities|FlowControl|Sequence
    (:then_0
      (Utilities|IsValid _weaponstaticmesh
        (:Is%20Valid
          (Components|DestroyComponent (Variables|Default|GetSkeletalMesh))
          (Components|StaticMesh|SetStaticMesh _staticmesh 0)
          (Transformation|SetRelativeLocation _staticmesh _location false false))
        (:Is%20Not%20Valid
          (Utilities|IsValid _weaponskeletmesh
            (:Is%20Valid
              (Components|DestroyComponent (Variables|Default|GetStaticMesh))
              (Class|SkinnedMeshComponent|SetSkeletalMesh _skeletalmesh 0 true)
              (Transformation|SetRelativeLocation _skeletalmesh _location false false))))))
    (:then_1
      (Utilities|IsValid _particlesystem
        (:Is%20Valid
          (Effects|Components|ParticleSystem|SetTemplate _particlesystem_2 0)
          (Transformation|SetRelativeScale3D _particlesystem_2 _scale))
        (:Is%20Not%20Valid
          (Components|DestroyComponent _particlesystem_2))))))