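; Ammo pickup actor that gives a character ammo for its configured weapon type when overlapped.
; On BeginPlay, InitActor selects a static mesh and particle effect by ammo type, destroying either component when no asset is mapped.
; The parent's OverlapCharacter event checks that the inventory can take that ammo, adds the count to its ammo slot, then signals pickup success.
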(event EventBeginPlay
  (|CallParentFunction)
  (CallFunction|InitActor))

(event Collision|EventActorBeginOverlap
  (params (OtherActor :type Actor%20Object%20Reference))
  (|CallParentFunction OtherActor) ; This node is disabled and will not be called.\nDrag off pins to build functionality.
)

(event EventTick
  (params (DeltaSeconds :type Float%20%28single-precision%29))
  (|CallParentFunction DeltaSeconds) ; This node is disabled and will not be called.\nDrag off pins to build functionality.
)

(event EventOverlapCharacter
  (params (ToInventory :type Top%20Down%20Shooter%20Inventor%20Component%20Object%20Reference))
  (bind _weapontypeammo (Variables|Default|GetWeaponTypeAmmo))
  (|CallParentFunction ToInventory)
  (bind _returnvalue (Class|TopDownShooterInventorComponent|CheckCanTakeAmmo ToInventory _weapontypeammo))
  (if _returnvalue
    (Class|TopDownShooterInventorComponent|AmmoSlotChangeValue ToInventory _weapontypeammo (Variables|Default|GetCout))
    (Default|PickUpSucces self)))

(fn ConstructionScript
  (|CallParentFunction))

(fn InitActor
  (bind _particlesystem (Variables|Default|GetParticleSystem))
  (bind _staticmesh (Variables|Default|GetStaticMesh))
  (bind _weapontypeammo (Variables|Default|GetWeaponTypeAmmo))
  (Utilities|FlowControl|Sequence
    (:then_0
      (Utilities|IsValid (Utilities|Select :Index _weapontypeammo :RifleType "/Game/Weapons/Assault_Rifle/Pickups/AssaultRifle_Pickup.AssaultRifle_Pickup" :AK47Type 0 :ShotGunType "/Game/Weapons/Shotgun/Sound/Wavs/Shotgun_AmmoPickup.Shotgun_AmmoPickup" :GrenadeLauncherType "/Game/Weapons/Grenade_Launcher/GrenadeLauncher_Pickup.GrenadeLauncher_Pickup")
        (:Is%20Valid
          (Components|StaticMesh|SetStaticMesh _staticmesh 0)
          (Transformation|SetRelativeLocation _staticmesh "0, 0, 0" false false)
          (Transformation|SetRelativeScale3D _staticmesh "2.000000,2.000000,2.000000")
          (Transformation|SetRelativeRotation _staticmesh (Utilities|Select :Index _weapontypeammo :RifleType "1.000000,1.000000,1.000000" :AK47Type "1.000000,1.000000,1.000000" :ShotGunType "1.000000,1.000000,1.000000" :GrenadeLauncherType "1.000000,1.000000,1.000000") false false))
        (:Is%20Not%20Valid
          (Components|DestroyComponent _staticmesh))))
    (:then_1
      (Utilities|IsValid (Utilities|Select :Index _weapontypeammo :RifleType "/Game/InfinityBladeEffects/Effects/FX_Mobile/ICE/combat/P_MagicSpray_Ice_00.P_MagicSpray_Ice_00" :AK47Type 0 :ShotGunType 0 :GrenadeLauncherType 0)
        (:Is%20Valid
          (Effects|Components|ParticleSystem|SetTemplate _particlesystem 0)
          (Transformation|SetRelativeScale3D _particlesystem "1.000000,1.000000,1.000000"))
        (:Is%20Not%20Valid
          (Components|DestroyComponent _particlesystem))))))